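; BP_LeafSpline is a procedural vine that builds a leaf-covered spline in the construction script.
; Each segment gets a spline mesh that follows the point tangents, its scale interpolated linearly from StartScale to EndScale.
; Instanced leaves are spaced along the spline by mesh X size plus Offset, oriented by tangent with AngleOffset added to Z.
; Leaf placement runs inside the segment loop, so the full set repeats per segment.
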(fn `GetLocationAtIndex`
  (params (A :type Integer))
  (returns (ReturnValue :type "Vector Structure"))
  (return (`SplineComponent.GetLocationAtDistanceAlongSpline` (`self.Spline`) (* A (`self.Spacing`)) "Local")))

(fn `UserConstructionScript`
  (locals (`Number of Instances` :type Integer :default 0))
  (bind _spline (`self.Spline`))
  (bind _start_scale (`self.Start Scale`))
  (bind (_min _max) (break `Box` (`StaticMesh.GetBoundingBox` (`self.Leaf`))))
  (bind _returnvalue (- (`SplineComponent.GetNumberOfSplinePoints` (`self.Spline`)) 2))
  (bind _returnvalue_2 (/ (- _start_scale (`self.End Scale`)) (`KismetMathLibrary.Conv_IntToDouble` (+ _returnvalue 1))))
  (for _index (range (+ _returnvalue 1))
    (bind _returnvalue_3 (`AddComponent|NODE_AddSplineMeshComponent-0`))
    (bind _returnvalue_4 (- _start_scale (* _index _returnvalue_2)))
    (`SplineMeshComponent.SetStartScale` _returnvalue_3 (`KismetMathLibrary.MakeVector2D` _returnvalue_4 _returnvalue_4) true)
    (bind _returnvalue_5 (- _start_scale (* (+ _index 1) _returnvalue_2)))
    (`SplineMeshComponent.SetEndScale` _returnvalue_3 (`KismetMathLibrary.MakeVector2D` _returnvalue_5 _returnvalue_5) true)
    (`StaticMeshComponent.SetStaticMesh` _returnvalue_3 (`self.Vine`))
    (`SplineMeshComponent.SetForwardAxis` _returnvalue_3 "X" true)
    (bind _returnvalue_6 (+ _index 1))
    (`SplineMeshComponent.SetStartAndEnd` _returnvalue_3 (`SplineComponent.GetLocationAtSplinePoint` _spline _index "Local") (`SplineComponent.GetTangentAtSplinePoint` _spline _index "Local") (`SplineComponent.GetLocationAtSplinePoint` _spline _returnvalue_6 "Local") (`SplineComponent.GetTangentAtSplinePoint` _spline _returnvalue_6 "Local") true)
    ;[1 1 1] Spawn Leaves
    (`StaticMeshComponent.SetStaticMesh` (`self.InstancedStaticMesh`) (`self.Leaf`))
    (bind _output_get (set `self.Spacing` (+ (.x (- _max _min)) (`self.Offset`))))
    (bind _output_get_2 (set `local.Number of Instances` (`KismetMathLibrary.FFloor` (/ (`SplineComponent.GetSplineLength` (`self.Spline`)) _output_get))))
    (for _index_2 (range (+ _output_get_2 1))
      (`InstancedStaticMeshComponent.AddInstance` (`self.InstancedStaticMesh`) (`KismetMathLibrary.MakeTransform` (`self.GetLocationAtIndex` _index_2) (`KismetMathLibrary.MakeRotFromX` (`KismetMathLibrary.MakeVector` (.x (`SplineComponent.GetTangentAtDistanceAlongSpline` (`self.Spline`) (* _index_2 _output_get) "Local")) (.y (`SplineComponent.GetTangentAtDistanceAlongSpline` (`self.Spline`) (* _index_2 _output_get) "Local")) (+ (.z (`SplineComponent.GetTangentAtDistanceAlongSpline` (`self.Spline`) (* _index_2 _output_get) "Local")) (`self.Angle Offset`)))))))))